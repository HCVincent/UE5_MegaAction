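; Base enemy Blueprint that handles defeat, destruction feedback and turning for enemy characters.
; On BeginPlay it binds to a defeated event, which destroys the actor.
; Destruction spawns a VFX actor and plays a defeat sound at the enemy's location, unless the enemy is being force-despawned.
; A TurnCharacter function flips the actor by combining its current rotation with a half-turn.
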(event `self.ReceiveBeginPlay`
  (`parent.ReceiveBeginPlay`)
  (add `self.Defeated` (delegate `OnDefeated`)))

(event `OnDefeated`
  (`self.K2_DestroyActor`))

(event `self.ReceiveDestroyed`
  (if (not (`self.IsBeingForceDespawned`))
    (`|SpawnActorFromClass` "/Game/Blueprints/VFX/BP_VFX_EnemyDestroyed.BP_VFX_EnemyDestroyed_C" (`KismetMathLibrary.MakeTransform` (`self.K2_GetActorLocation`) (`self.K2_GetActorRotation`)) "AlwaysSpawn" "MultiplyWithRoot" null null)
    (`GameplayStatics.PlaySoundAtLocation` "/Game/Audio/SFX/Enemy_Defeat_Cue.Enemy_Defeat_Cue" (`self.K2_GetActorLocation`) (struct) 1.0 1.0 0.0 null null null null)))

(fn `TurnCharacter`
  (`self.K2_SetActorRotation` (`KismetMathLibrary.ComposeRotators` (`self.K2_GetActorRotation`) (struct :`Yaw` 180.0))))

(fn `UserConstructionScript`
  (`parent.UserConstructionScript`))